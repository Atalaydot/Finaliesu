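; Unit actor Blueprint that highlights on mouse hover and can raise or lower its Box component.
; Cursor over Box applies a Glow overlay material to Cube1, and clicking Cube1 clears it.
; The Geldi event, not called within this graph, uses DoOnce and FlipFlop to alternate eased one-second moves down and back, re-arming after each move.
; Debug prints remain, along with an unconnected SetActive toggle.
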(event `Geldi`
  (bind _box (`self.Box`))
  (`/Engine/EditorBlueprintResources/StandardMacros.DoOnce` false :!label _label
    (:`Completed`
      (`/Engine/EditorBlueprintResources/StandardMacros.FlipFlop`
        (:`A`
          (`KismetSystemLibrary.MoveComponentTo` _box (0.0 0.0 -100.0) (struct) true true 1.0)
          (`KismetSystemLibrary.PrintText` "FFF")
          (goto _label :!via `Reset`))
        (:`B`
          (`KismetSystemLibrary.MoveComponentTo` _box (0.0 0.0 0.0) (struct) true true 1.0)
          (`KismetSystemLibrary.PrintText` "sss")
          (goto _label :!via `Reset`))))))

(event `deneme`
  (`MeshComponent.SetOverlayMaterial` (`self.Cube1`) "/Game/Material/glow.glow"))

(event `self.Box.OnBeginCursorOver`
  (params (TouchedComponent :type "PrimitiveComponent Object Reference"))
  (`self.deneme`)
  (`KismetSystemLibrary.PrintText` "Hello"))

(event `Denem2`
  (`MeshComponent.SetOverlayMaterial` (`self.Cube1`) null))

(event `self.Cube1.OnClicked`
  (params (TouchedComponent :type "PrimitiveComponent Object Reference") (ButtonPressed :type "Key Structure"))
  (`self.Denem2`))

(fn `UserConstructionScript`)