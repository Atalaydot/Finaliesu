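; BP_camera2 is a trigger volume that switches the third-person character to the second of four camera states.
; When the character enters the Box, it calls SecondLock, sets only the Second flag true, and eases the CameraBoom to a fixed relative rotation with MoveComponentTo.
; BeginPlay caches the first BP_camera2 found in Camere2, but the view-target blend that uses it is disconnected and never runs.
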(event `self.ReceiveBeginPlay`
  (bind _returnvalue (`GameplayStatics.GetActorOfClass` "BP_camera2_C"))
  (set `/Game/Bp/BP_camera2.Camere2` _returnvalue _returnvalue))

(event `self.Box.OnComponentBeginOverlap`
  (params (OverlappedComponent :type "PrimitiveComponent Object Reference") (OtherActor :type "Actor Object Reference") (OtherComp :type "PrimitiveComponent Object Reference") (OtherBodyIndex :type Integer) (bFromSweep :type Boolean) (SweepResult :type "HitResult Structure (by ref)"))
  (bind _asbp_third_person_character (cast `/Game/ThirdPerson/Blueprints/BP_ThirdPersonCharacter` OtherActor))
  (`/Game/ThirdPerson/Blueprints/BP_ThirdPersonCharacter.SecondLock` _asbp_third_person_character)
  (set `/Game/ThirdPerson/Blueprints/BP_ThirdPersonCharacter.First` false _asbp_third_person_character)
  (set `/Game/ThirdPerson/Blueprints/BP_ThirdPersonCharacter.Second` true _asbp_third_person_character)
  (set `/Game/ThirdPerson/Blueprints/BP_ThirdPersonCharacter.Third` false _asbp_third_person_character)
  (set `/Game/ThirdPerson/Blueprints/BP_ThirdPersonCharacter.Four` false _asbp_third_person_character)
  (`KismetSystemLibrary.MoveComponentTo` (`/Game/ThirdPerson/Blueprints/BP_ThirdPersonCharacter.CameraBoom` _asbp_third_person_character) (0.0 0.0 0.0) (struct :`Yaw` -90.0) true true 1.0))

(fn `UserConstructionScript`)